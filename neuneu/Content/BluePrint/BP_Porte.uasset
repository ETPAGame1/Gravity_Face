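; Door Blueprint whose static mesh rises and returns in response to the I_pression and I_END events, likely from pressure plates.
; I_pression stores the mesh location and plays the OpenDoor timeline, while I_END plays Timeline_0 back toward that stored location.
; Both lerp from the current location each update, so the raise compounds beyond its nominal Z offset.
; Only index 0 moves the mesh; other indices just print debug text.
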(event Custom|I_pression
  (params (Num_PP :type Integer))
  (bind _staticmesh (Variables|Default|GetStaticMesh))
  (bind _returnvalue (Transformation|GetWorldLocation _staticmesh))
  (Variables|Default|Setvalue%20start _returnvalue)
  (bind _newtrack_0 (Timeline|Open%20door PlayFromStart)
    (:Update
      (switch int Num_PP
        (:Default
          (Development|PrintString "marche mais pas vraiment"))
        (:0
          (Transformation|SetWorldLocation (Variables|Default|GetStaticMesh) (Math|Vector|Lerp(Vector) _returnvalue (+ _returnvalue "0.000000,0.000000,100.000000") _newtrack_0) false false))
        (:1
          (Development|PrintString "1"))
        (:2
          (Development|PrintString "2"))))))

(event Custom|I_END
  (params (Num_pp_End :type Integer))
  (bind _newtrack_0 (Timeline|Timeline_0 PlayFromStart)
    (:Update
      (switch int Num_pp_End
        (:Default
          (Development|PrintString "marche mais pas vraiment"))
        (:0
          (Development|PrintString "pute")
          (Transformation|SetWorldLocation (Variables|Default|GetStaticMesh) (Math|Vector|Lerp(Vector) (Transformation|GetWorldLocation (Variables|Default|GetStaticMesh)) (Variables|Default|Getvalue%20start) _newtrack_0) false false))))))

(fn ConstructionScript)