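; BP_Ball is a ball actor that other code can pick up and release.
; Attach parents it to a supplied WorldPivot component, keeping its world transform, and switches off physics and gravity on its Sphere.
; Detach frees it from its parent, zeroes linear velocity, then restores physics and gravity, so it drops without carried momentum.
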(event EventDetach
  (bind _sphere (Variables|Default|GetSphere))
  (Transformation|DetachFromActor "KeepWorld" "KeepWorld" "KeepWorld")
  (Class|PrimitiveComponent|SetAllPhysicsLinearVelocity (Variables|Default|GetSphere) "0, 0, 0" false)
  (Physics|SetSimulatePhysics _sphere true)
  (Physics|SetEnableGravity _sphere true))

(event EventAttach
  (params (WorldPivot :type Scene%20Component%20Object%20Reference))
  (bind _sphere (Variables|Default|GetSphere))
  (Transformation|AttachComponentToComponent WorldPivot "None" "KeepWorld" "KeepWorld" "KeepWorld" true)
  (Physics|SetSimulatePhysics _sphere false)
  (Physics|SetEnableGravity _sphere false))

(fn ConstructionScript)