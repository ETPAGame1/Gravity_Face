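; Pressure plate that opens its linked doors while something stands on it.
; Box begin overlap calls OpenDoor on every entry in PortesRef and end overlap calls CloseDoor, with no actor filtering or overlap counting.
; The construction script adds one spline per door, ending at that door's location, so the links are drawn from the plate.
; An Attach event parents the plate to a given world pivot, keeping its world transform.
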(event OnComponentBeginOverlap(Box)
  (params (OverlappedComponent :type Primitive%20Component%20Object%20Reference) (OtherActor :type Actor%20Object%20Reference) (OtherComp :type Primitive%20Component%20Object%20Reference) (OtherBodyIndex :type Integer) (bFromSweep :type Boolean) (SweepResult :type Hit%20Result%20Structure%20%28by%20ref%29))
  (Development|PrintString "overlaps")
  (for _array_element (Variables|Default|GetPortesRef)
    (Default|OpenDoor _array_element)))

(event OnComponentEndOverlap(Box)
  (params (OverlappedComponent :type Primitive%20Component%20Object%20Reference) (OtherActor :type Actor%20Object%20Reference) (OtherComp :type Primitive%20Component%20Object%20Reference) (OtherBodyIndex :type Integer))
  (for _array_element (Variables|Default|GetPortesRef)
    (Default|CloseDoor _array_element)))

(event EventAttach
  (params (WorldPivot :type Scene%20Component%20Object%20Reference))
  (Transformation|AttachComponentToComponent WorldPivot "None" "KeepWorld" "KeepWorld" "KeepWorld" true))

(fn ConstructionScript
  (for _array_element (Variables|Default|GetPortesRef)
    (bind _returnvalue (AddComponent|AddSplineComponent false))
    (Spline|SetLocationatSplinePoint _returnvalue 1 (Transformation|GetActorLocation _array_element) "World" true)))