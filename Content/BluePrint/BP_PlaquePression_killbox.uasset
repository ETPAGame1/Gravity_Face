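; Pressure plate Blueprint that destroys its referenced BP_KillBox actors when the first-person character steps on it.
; The box overlap identifies the player by comparing the component display name to a hardcoded string, printing debug text along the way.
; An Attach event parents it to a given WorldPivot, keeping world transform.
; The construction script adds a spline component per array element, placing its second point at that actor's location.
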(event OnComponentBeginOverlap(Box)
  (params (OverlappedComponent :type Primitive%20Component%20Object%20Reference) (OtherActor :type Actor%20Object%20Reference) (OtherComp :type Primitive%20Component%20Object%20Reference) (OtherBodyIndex :type Integer) (bFromSweep :type Boolean) (SweepResult :type Hit%20Result%20Structure%20%28by%20ref%29))
  (bind _returnvalue (Utilities|GetDisplayName OtherComp))
  (Development|PrintString _returnvalue)
  (if (Utilities|Enum|Equal(Enum) _returnvalue "FirstPersonCharacter_C_0.CollisionCylinder")
    (for _array_element (Variables|Default|GetKillBoxRef)
      (bind _asbp_kill_box (Utilities|Casting|CastToBP_KillBox _array_element))
      (Actor|DestroyActor _asbp_kill_box))
    (else
      (Development|PrintString "Hello"))))

(event EventAttach
  (params (WorldPivot :type Scene%20Component%20Object%20Reference))
  (Transformation|AttachComponentToComponent WorldPivot "None" "KeepWorld" "KeepWorld" "KeepWorld" true))

(fn ConstructionScript
  (for _array_element 0
    (bind _returnvalue (AddComponent|AddSplineComponent false))
    (Spline|SetLocationatSplinePoint _returnvalue 1 (Transformation|GetActorLocation _array_element) "World" true)))