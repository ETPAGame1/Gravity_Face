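; Ball Blueprint whose Sphere component can be attached to a pivot and switched in and out of physics simulation.
; An Attach event parents a component to the supplied WorldPivot, keeping world transforms.
; Separate attach and detach events toggle gravity and physics, printing French debug messages.
; Tick re-enables both gravity and physics every frame, which overrides the disabling done by attach_ball.
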(event Custom|attach_ball
  (bind _sphere (Variables|Default|GetSphere))
  (Physics|SetSimulatePhysics _sphere false)
  (Physics|SetEnableGravity _sphere false)
  (Development|PrintString "plus de physique"))

(event Custom|detach_ball
  (bind _sphere (Variables|Default|GetSphere))
  (Physics|SetSimulatePhysics _sphere true)
  (Physics|SetEnableGravity _sphere true)
  (Development|PrintString "de nouveau de la physique"))

(event EventTick
  (params (DeltaSeconds :type Float%20%28single-precision%29))
  (Physics|SetEnableGravity (Variables|Default|GetSphere) true)
  (Physics|SetSimulatePhysics (Variables|Default|GetSphere) true))

(event EventAttach
  (params (WorldPivot :type Scene%20Component%20Object%20Reference))
  (Transformation|AttachComponentToComponent WorldPivot "None" "KeepWorld" "KeepWorld" "KeepWorld" true))

(fn ConstructionScript)