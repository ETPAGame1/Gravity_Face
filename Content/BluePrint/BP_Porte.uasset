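; BP_Porte is a door Blueprint that swings open and closed by rotating its root component in yaw.
; BeginPlay stores the starting relative yaw, and a timeline lerps from it to 90 degrees beyond, keeping roll and pitch.
; OpenDoor plays the timeline and CloseDoor reverses it.
; An Attach event parents the door to a supplied WorldPivot, keeping its world transform.
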(event Custom|OpenDoor
  (bind _defaultsceneroot (Variables|Default|GetDefaultSceneRoot))
  (bind _value_start (Variables|Default|Getvalue%20start))
  (bind _relativerotation (Variables|/Script/Engine.SceneComponent|GetRelativeRotation _defaultsceneroot))
  (bind _newtrack_0 (Timeline|Open%20door Play)
    (:Update
      (Transformation|SetRelativeRotation (Variables|Default|GetDefaultSceneRoot) (Math|Rotator|MakeRotator (.roll _relativerotation) (.pitch _relativerotation) (Math|Float|Lerp _value_start (+ _value_start 9e+01) _newtrack_0)) false false))))

(event Custom|CloseDoor
  (bind _defaultsceneroot (Variables|Default|GetDefaultSceneRoot))
  (bind _value_start (Variables|Default|Getvalue%20start))
  (bind _relativerotation (Variables|/Script/Engine.SceneComponent|GetRelativeRotation _defaultsceneroot))
  (bind _newtrack_0 (Timeline|Open%20door Reverse)
    (:Update
      (Transformation|SetRelativeRotation (Variables|Default|GetDefaultSceneRoot) (Math|Rotator|MakeRotator (.roll _relativerotation) (.pitch _relativerotation) (Math|Float|Lerp _value_start (+ _value_start 9e+01) _newtrack_0)) false false))))

(event EventAttach
  (params (WorldPivot :type Scene%20Component%20Object%20Reference))
  (Transformation|AttachComponentToComponent WorldPivot "None" "KeepWorld" "KeepWorld" "KeepWorld" true))

(event EventBeginPlay
  (Variables|Default|Setvalue%20start (.yaw (Variables|/Script/Engine.SceneComponent|GetRelativeRotation (Variables|Default|GetDefaultSceneRoot)))))

(fn ConstructionScript)